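; Inventory component for the first-person character that finds items in view, triggers their interaction and stores item row names.
; Each tick a debug-drawn sphere trace from the camera updates LookAtActor.
; The interaction input passes the owning character to that actor's BP_ItemData component through InteractWithMessage.
; AddToInventory adds unique row names up to three slots, ignores its DataTable input, and prints a message when full.
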(event Custom|Interact
  (params (Actor :type Actor%20Object%20Reference))
  (bind _returnvalue (Actor|GetComponentbyClass Actor "/Game/Core/Blueprints/Inventory/BP_ItemData.BP_ItemData_C"))
  (Utilities|IsValid _returnvalue
    (:Is%20Valid
      (Class|IInteractInterface|Interactwith(Message) _returnvalue (.AsBP%20First%20Person%20Character (Utilities|Casting|CastToBP_FirstPersonCharacter (Components|GetOwner)))))))

(event Input|EnhancedActionEvents|EnhancedInputActionIA_Interaction
  (params (ActionValue :type Boolean) (ElapsedSeconds :type Float%20%28double-precision%29) (TriggeredSeconds :type Float%20%28double-precision%29) (InputAction :type Input%20Action%20Object%20Reference :default "/Game/FirstPerson/Input/Actions/IA_Interaction.IA_Interaction"))
  (bind _lookatactor (Variables|Default|GetLookAtActor)
    (:then
      (CallFunction|Interact _lookatactor))
    (:else)))

(event EventTick
  (params (DeltaSeconds :type Float%20%28single-precision%29))
  (CallFunction|InteractTrace))

(fn AddtoInventory
  (params (DataTable :type Data%20Table%20Object%20Reference) (Row%20Name :type Name))
  (if (< (Utilities|Array|Length (Variables|Default|GetItemArr)) 3)
    (Utilities|Array|AddUnique (Variables|Default|GetItemArr) Row%20Name)
    (return true)
    (else
      (Development|PrintString "IventoryFull")
      (return false))))

(fn InteractTrace
  (bind _returnvalue (Game|GetPlayerCameraManager 0))
  (bind _returnvalue_2 (Transformation|GetActorLocation _returnvalue))
  (bind (_outhit _returnvalue_3) (Collision|SphereTraceByChannel _returnvalue_2 (+ _returnvalue_2 (* (Math|Vector|GetForwardVector (Variables|/Script/Engine.PlayerCameraManager|GetTransformComponent _returnvalue)) (Variables|Default|GetInteractionRange))) 15.0 "TraceTypeQuery3" false (Utilities|Array|MakeArray (Components|GetOwner)) "ForOneFrame"))
  (if _returnvalue_3
    (if (!= (.HitActor (Collision|BreakHitResult _outhit)) (Variables|Default|GetLookAtActor))
      (Variables|Default|SetLookAtActor (.HitActor (Collision|BreakHitResult _outhit))))
    (else
      (Variables|Default|SetLookAtActor 0))))